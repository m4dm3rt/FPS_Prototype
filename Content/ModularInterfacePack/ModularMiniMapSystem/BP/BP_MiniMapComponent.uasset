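; Player controller component that drives a top-down minimap by creating a render target and spawning a scene capture actor for the local player.
; Each tick it moves the capture actor above the controlled pawn, or the camera without one, with yaw fixed or following the pawn or camera.
; It announces the new render target and exposes events to change ortho width and hide or clear hidden actors and components on the map.
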(event Custom|SetOrthoWidth
  (params (NewOrthoWidth :type Float%20%28double-precision%29))
  ;[1 1 1] Comment
  (bind _output_get (Variables|Default|SetOrthoWidth NewOrthoWidth))
  (bind _minimapcaptureactor (Variables|Default|GetMiniMapCaptureActor)
    (:then
      (bind _output_get_2 (Variables|/Game/ModularInterfacePack/ModularMiniMapSystem/BP/BP_MiniMapCaptureActor.BP_MiniMapCaptureActor_C|SetWidth _minimapcaptureactor _output_get))
      (Variables|/Script/Engine.SceneCaptureComponent2D|SetOrthoWidth (Variables|/Script/Engine.SceneCapture2D|GetCaptureComponent2D _minimapcaptureactor) _output_get_2))
    (:else)))

(event Custom|HideActorsOnMiniMap
  (params (InActor :type Actor%20Object%20Reference) (bIncludeFromChildActors :type Boolean))
  (bind _capture_component_2d (CallFunction|GetCaptureComponent))
  (Utilities|IsValid _capture_component_2d
    (:Is%20Valid
      (Class|SceneCaptureComponent|HideActorComponents _capture_component_2d InActor bIncludeFromChildActors))))

(event Custom|HideComponentOnMiniMap
  (params (InComponent :type Primitive%20Component%20Object%20Reference))
  (bind _capture_component_2d (CallFunction|GetCaptureComponent))
  (Utilities|IsValid _capture_component_2d
    (:Is%20Valid
      (Class|SceneCaptureComponent|HideComponent _capture_component_2d InComponent))))

(event Custom|ClearHiddenComponentsOnMiniMap
  (bind _capture_component_2d (CallFunction|GetCaptureComponent))
  (Utilities|IsValid _capture_component_2d
    (:Is%20Valid
      (Class|SceneCaptureComponent|ClearHiddenComponents _capture_component_2d))))

(event EventBeginPlay
  (bind _resolution (Variables|Default|GetResolution))
  ;[1 1 1] Comment
  (bind _asplayer_controller (Utilities|Casting|CastToPlayerController (Components|GetOwner))
    (:then
      (bind _output_get (Variables|Default|SetPlayerController _asplayer_controller))
      (if (Pawn|IsLocalController _output_get)
        (bind _returnvalue (Rendering|CreateRenderTarget2D _resolution _resolution "RTF_RGBA16f"))
        (bind _output_get_2 (Variables|Default|SetRenderTargetTexture _returnvalue))
        (Default|CallOnRenderTargetTextureCreated _output_get_2)
        (bind _returnvalue_2 (Game|SpawnActorfromClass "/Game/ModularInterfacePack/ModularMiniMapSystem/BP/BP_MiniMapCaptureActor.BP_MiniMapCaptureActor_C" (Math|Transform|MakeTransform (Camera|GetCameraLocation (Variables|/Script/Engine.PlayerController|GetPlayerCameraManager (Variables|Default|GetPlayerController))) (Camera|GetCameraRotation (Variables|/Script/Engine.PlayerController|GetPlayerCameraManager (Variables|Default|GetPlayerController))) "1.000000,1.000000,1.000000") "AlwaysSpawn" "MultiplyWithRoot" (Variables|Default|GetPlayerController) (Variables|Default|GetOrthoWidth) (Variables|Default|GetRenderTargetTexture) (Variables|Default|GetSceneCaptureSource) (Variables|Default|GetPostProcessMaterial) 0))
        (Variables|Default|SetMiniMapCaptureActor _returnvalue_2)))
    (:CastFailed
      (Development|PrintString "BP MINIMAP COMPONENT ONLY FOR CONTROLLER"))))

(event EventTick
  (params (DeltaSeconds :type Float%20%28single-precision%29))
  ;[1 1 1] Comment
  (bind _location (CallFunction|GetPlayerPosition))
  (bind _minimapcaptureactor (Variables|Default|GetMiniMapCaptureActor)
    (:then
      (Transformation|SetActorLocation _minimapcaptureactor (+ _location (Math|Vector|MakeVector 0.0 0.0 (Variables|Default|GetCameraHeight))) false false)
      (bind _yaw (CallFunction|GetCaptureRotation))
      (Transformation|SetActorRotation _minimapcaptureactor (Math|Rotator|MakeRotator 0.0 0.0 _yaw)))
    (:else)))

(fn GetPlayerPosition
  (bind _playercontroller (Variables|Default|GetPlayerController)
    (:then
      (Utilities|IsValid (Pawn|GetControlledPawn _playercontroller)
        (:Is%20Valid
          (return (Transformation|GetActorLocation (Pawn|GetControlledPawn _playercontroller))))
        (:Is%20Not%20Valid
          (return (Camera|GetCameraLocation (Variables|/Script/Engine.PlayerController|GetPlayerCameraManager _playercontroller))))))
    (:else
      (return "0, 0, 0"))))

(fn GetCaptureRotation
  (switch Utilities|FlowControl|Switch|SwitchonE_MM_CaptureRotationMode (Variables|Default|GetCaptureRotationMode)
    (:NewEnumerator0
      _)
    (:NewEnumerator1
      (bind _playercontroller (Variables|Default|GetPlayerController)
        (:then
          (Utilities|IsValid (Pawn|GetControlledPawn _playercontroller)
            (:Is%20Valid
              (return (.Yaw (Math|Rotator|BreakRotator (Transformation|GetActorRotation (Pawn|GetControlledPawn _playercontroller))))))
            (:Is%20Not%20Valid
              (return (.Yaw (Math|Rotator|BreakRotator (Camera|GetCameraRotation (Variables|/Script/Engine.PlayerController|GetPlayerCameraManager _playercontroller))))))))
        (:else
          _)))
    (:NewEnumerator2
      (bind _playercontroller_2 (Variables|Default|GetPlayerController)
        (:then
          (return (.Yaw (Math|Rotator|BreakRotator (Camera|GetCameraRotation (Variables|/Script/Engine.PlayerController|GetPlayerCameraManager _playercontroller_2))))))
        (:else
          _))))
  (return 0.0))

(fn GetCaptureComponent
  (bind _minimapcaptureactor (Variables|Default|GetMiniMapCaptureActor)
    (:then
      (return (Variables|/Script/Engine.SceneCapture2D|GetCaptureComponent2D _minimapcaptureactor)))
    (:else
      (return 0))))