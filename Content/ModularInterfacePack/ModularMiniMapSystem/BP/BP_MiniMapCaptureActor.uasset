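; BP_MiniMapCaptureActor is a scene capture actor for the modular minimap system that captures the scene into a render target.
; On BeginPlay it configures its SceneCaptureComponent2D with the ortho width, target texture and capture source held in its variables.
; If a post-process material is valid, it applies it at full weight as a weighted blendable in the capture's post-process settings.
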(event EventBeginPlay
  ;[1 1 1] Comment
  (Variables|/Script/Engine.SceneCaptureComponent2D|SetOrthoWidth (Variables|DecalActor|GetCaptureComponent2D) (Variables|Default|GetWidth))
  (Variables|/Script/Engine.SceneCaptureComponent2D|SetTextureTarget (Variables|DecalActor|GetCaptureComponent2D) (Variables|Default|GetRenderTargetTexture))
  (Variables|/Script/Engine.SceneCaptureComponent|SetCaptureSource (Variables|DecalActor|GetCaptureComponent2D) (Variables|Default|GetSceneCaptureSource))
  (bind _postprocessmaterial (Variables|Default|GetPostProcessMaterial)
    (:then
      (Utilities|Struct|SetmembersinPostProcessSettings (Variables|/Script/Engine.SceneCaptureComponent2D|GetPostProcessSettings (Variables|DecalActor|GetCaptureComponent2D)) (Utilities|Struct|MakeWeightedBlendables (Utilities|Array|MakeArray (Utilities|Struct|MakeWeightedBlendable 1.0 _postprocessmaterial)))))
    (:else)))

(fn ConstructionScript)