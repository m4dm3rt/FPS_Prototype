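; Demo player character that connects weapon equip, fire and fire-mode events to a procedural RecoilAnimation component.
; Locally controlled pawns use a separate TFP mannequin mesh to hide the head, and debug keys toggle camera shake and the recoil UI.
; In edit mode, number keys change weapon attachments, rescaling recoil input around each edit.
; Client edits go through a server event and multicast to non-local copies.
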(event Custom|Multicast_OnAttachmentEdited
  (params (Index :type Integer))
  ;[0 1 0.1014] Attachment editing
  (if (not (Pawn|IsLocallyControlled))
    (CallFunction|OnAttachmentEdited Index)))

(event Custom|Server_OnAttachmentEdited
  (params (Index :type Integer))
  ;[0 1 0.1014] Attachment editing
  (if (Ability|HasAuthority)
    (CallFunction|MulticastonAttachmentEdited Index)))

(event EventBeginPlay
  (bind _mesh (Variables|Character|GetMesh))
  ;[0.1263 0.8943 1] Hide head mesh on local client
  (if (Pawn|IsLocallyControlled)
    (Components|SkinnedMesh|SetSkinnedAssetandUpdate _mesh "/Game/Animations/UE4_Mannequin/Mesh/SK_Mannequin_TFP.SK_Mannequin_TFP" false)
    (else
      (Components|SkinnedMesh|SetSkinnedAssetandUpdate _mesh "/Game/Animations/UE4_Mannequin/Mesh/SK_Mannequin.SK_Mannequin" false))))

(event EventTick
  (params (DeltaSeconds :type Float%20%28single-precision%29))
  ;[0.8741 0.4417 1] Current fire mode
)

(event EventOnWeaponEquipped
  (params (Data :type Recoil%20Anim%20Data%20Structure) (Rate :type Float%20%28single-precision%29) (Bursts :type Integer))
  ;[0.01309 1 0] Call Init whenever weapon is equipped
  (Class|RecoilAnimationComponent|Init (Variables|Default|GetRecoilAnimation) Data Rate Bursts))

(event EventOnFirePressed
  ;[0.01309 1 0] Fire pressed/released
  (Class|RecoilAnimationComponent|Play (Variables|Default|GetRecoilAnimation)))

(event EventOnFireReleased
  ;[0.01309 1 0] Fire pressed/released
  (Class|RecoilAnimationComponent|Stop (Variables|Default|GetRecoilAnimation)))

(event EventOnFireModeChanged
  (params (NewMode :type EFireMode_PRAS%20Enum :default "Semi"))
  ;[0.01309 1 0] Fire mode update
  (Class|RecoilAnimationComponent|SetFireMode (Variables|Default|GetRecoilAnimation) NewMode))

(event Input|ActionEvents|InputActionToggleAttachments
  (params (Key :type Key%20Structure))
  ;[1 0.05117 0.5944] Weapon customization
  (:Pressed
    (Variables|Default|SetbEditing (not (Variables|Default|GetbEditing)))))

(event Input|ActionEvents|InputActionSelectAttachment
  (params (Key :type Key%20Structure))
  ;[0 1 0.1014] Attachment editing
  (:Pressed
    (if (Variables|Default|GetbEditing)
      (if (== Key "One")
        (CallFunction|OnAttachmentEdited)
        (elif (== Key "Two")
          (CallFunction|OnAttachmentEdited 1)
          (elif (== Key "Three")
            (CallFunction|OnAttachmentEdited 2)
            (elif (== Key "Four")
              (CallFunction|OnAttachmentEdited 3))))))))

(event Input|KeyboardEvents|LeftCtrl
  (params (Key :type Key%20Structure))
  (bind _recoilanimation (Variables|Default|GetRecoilAnimation))
  ;[0.01309 1 0] Helper UI
  (:Pressed
    (Utilities|FlowControl|FlipFlop
      (:A
        (Class|RecoilAnimationComponent|ShowUI _recoilanimation))
      (:B
        (Class|RecoilAnimationComponent|HideUI _recoilanimation)))))

(event Input|KeyboardEvents|LeftAlt
  (params (Key :type Key%20Structure))
  ;[0.01309 1 0] Toggle camera shake
  (:Pressed
    (Variables|Default|SetbEnableShake (not (Variables|Default|GetbEnableShake)))))

(fn ConstructionScript)

(fn OnAttachmentEdited
  (params (Index :type Integer))
  (bind _returnvalue (Class|PRASDemoProjectCharacter|GetWeapon))
  (Utilities|IsValid _returnvalue
    (:Is%20Valid
      (bind _returnvalue_2 (Class|Weapon|GetAnimScalefromGroup _returnvalue Index))
      (Class|RecoilAnimationComponent|UnscaleInput (Variables|Default|GetRecoilAnimation) _returnvalue_2)
      (Class|Weapon|EditAttachments _returnvalue Index)
      (bind _returnvalue_3 (Class|Weapon|GetAnimScalefromGroup _returnvalue Index))
      (Class|RecoilAnimationComponent|ScaleInput (Variables|Default|GetRecoilAnimation) _returnvalue_3)
      (if (not (Ability|HasAuthority))
        (CallFunction|ServeronAttachmentEdited Index)))))